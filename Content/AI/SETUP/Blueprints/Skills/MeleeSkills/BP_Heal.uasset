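; BP_Heal is a short-lived skill actor that restores Health to its owner, using the Damage value as the heal amount.
; On BeginPlay it updates player stats for BP_ParentAI owners, or writes BP_Enemy's stat array clamped to the enemy's maximum health.
; Tick keeps the effect on the owner's location until a brief delay deactivates it and destroys the skill.
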(event `self.ReceiveBeginPlay`
  (bind _skill_owner (`self.Skill_Owner`))
  ;[1 1 1] Used by player
  (cast `/Game/AI/SETUP/Blueprints/Character/BP_ParentAI` _skill_owner
    (:`then`
      (`/Game/AI/SETUP/Blueprints/Utility/BFL_UtilitiesLibrary.SetPlayersState` "Health" (+ (`/Game/AI/SETUP/Blueprints/Utility/BFL_UtilitiesLibrary.GetPlayersState` "Health") (`self.Damage`))))
    (:`CastFailed`
      ;[1 1 1] Used by enemy
      (bind _asbp_enemy (cast `/Game/AI/SETUP/Blueprints/AI/BP_Enemy` _skill_owner))
      (bind _statcurrent (`/Game/AI/SETUP/Blueprints/AI/BP_Enemy.StatCurrent` _asbp_enemy))
      (bind _returnvalue (`KismetArrayLibrary.Array_Find` (`/Game/AI/SETUP/Blueprints/AI/BP_Enemy.StatName` _asbp_enemy) "Health"))
      (`KismetArrayLibrary.Array_Set` _statcurrent _returnvalue (`KismetMathLibrary.FClamp` (+ (`|GetArrayItem` _statcurrent _returnvalue) (`self.Damage`)) 0.0 (`.EnemyHealth_27_6CA6BFE444881DE6D5D02A88DEE50FB7` (break `/Game/AI/SETUP/Blueprints/AI/Datatable/NPCStats` (`/Game/AI/SETUP/Blueprints/AI/BP_Enemy.NPCStats` _asbp_enemy)))))))
  ;[1 1 1] Deactivate effect after delay
  (`KismetSystemLibrary.Delay` 0.5)
  (`ActorComponent.Deactivate` (`self.Effect`))
  (`self.DestroySkill`))

(event `self.ReceiveTick`
  (params (DeltaSeconds :type "Float (single-precision)"))
  ;[1 1 1] Set location for effect
  (`self.K2_SetActorLocation` (`self.K2_GetActorLocation` (`self.Skill_Owner`))))

(fn `UserConstructionScript`
  (`parent.UserConstructionScript`))