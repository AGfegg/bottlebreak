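; BP_RingOfLight is a melee skill that sweeps a damaging light effect in a ring around its owner.
; Tick keeps the center on the owner, while a Rotation timeline drives the angle for circular line traces and the Niagara position.
; Depending on owner type, traces damage living enemies or the player via HitBox, once per target using HittedActors.
; The skill destroys itself when the timeline finishes.
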(event `self.ReceiveTick`
  (params (DeltaSeconds :type "Float (single-precision)"))
  ;[1 1 1] Updating center coordinate of ring
  (`parent.ReceiveTick` 0.0)
  (set `self.CenterPoint` (`self.K2_GetActorLocation` (`self.Skill_Owner`))))

(event `self.ReceiveBeginPlay`
  (bind _ringradius (`self.RingRadius`))
  (bind (_bblockinghit _binitialoverlap _time _distance _location _impactpoint _normal _impactnormal _physmat _hitactor _hitcomponent) (`GameplayStatics.BreakHitResult` (`self.NextHitResult`)))
  (bind (_direction _angle) (`Timeline|Rotation`)
    (:`Update`
      (bind _returnvalue (`KismetMathLibrary.MakeVector` (+ (* (`KismetMathLibrary.DegCos` _angle) _ringradius) (.x (`self.CenterPoint`))) (+ (* _ringradius (`KismetMathLibrary.DegSin` _angle)) (.y (`self.CenterPoint`))) (.z (`self.CenterPoint`))))
      ;[1 1 1] Damage for each unique enemy in range
      (bind _outhits (`KismetSystemLibrary.LineTraceMultiForObjects` (`self.CenterPoint`) _returnvalue (`|MakeArray` "ObjectTypeQuery2" :!type "EObjectTypeQuery Enum")))
      (for _array_element _outhits
        (set `self.NextHitResult` _array_element)
        ;;[1 1 1] Who is skill owner?
        (cast `/Game/AI/SETUP/Blueprints/Character/BP_ParentAI` (`self.Skill_Owner`)
          (:`then`
            ;;[1 1 1] Used by Player
            ;;;[1 1 1] Ignore all other actors
            (bind _asbp_enemy (cast `/Game/AI/SETUP/Blueprints/AI/BP_Enemy` (`ActorComponent.GetOwner` _hitcomponent)))
            (set `self.NextEnemy` _asbp_enemy)
            ;;;[1 1 1] If trace hit enemy's HitBox...
            (if (and (== (`/Game/AI/SETUP/Blueprints/AI/BP_Enemy.HitBox` (`self.NextEnemy`)) _hitcomponent) (not (`/Game/AI/SETUP/Blueprints/AI/BP_Enemy.EnemyIsDead` (`self.NextEnemy`))))
              ;;;[1 1 1] ...and it's first hit in this enemy...
              (if (== (`KismetArrayLibrary.Array_Find` (`self.HittedActors`) (`self.NextEnemy`)) -1)
                ;;;[1 1 1] apply damage.
                (`GameplayStatics.ApplyDamage` (`self.NextEnemy`) (`self.Damage`))
                (`KismetArrayLibrary.Array_AddUnique` (`self.HittedActors`) (`self.NextEnemy`)))))
          (:`CastFailed`
            ;;[1 1 1] Used by Enemy
            ;;;[1 1 1] If trace hit player's HitBox
            (if (== (`/Game/AI/SETUP/Blueprints/Utility/BFL_UtilitiesLibrary.GetPlayersHitBox`) (`.HitComponent` (`GameplayStatics.BreakHitResult` (`self.NextHitResult`))))
              ;;;[1 1 1] ...and it's first hit in player...
              (if (== (`KismetArrayLibrary.Array_Find` (`self.HittedActors`) (`/Game/AI/SETUP/Blueprints/Utility/BFL_UtilitiesLibrary.GetPlayer`)) -1)
                ;;;[1 1 1] ...apply damage
                (`GameplayStatics.ApplyDamage` (`/Game/AI/SETUP/Blueprints/Utility/BFL_UtilitiesLibrary.GetPlayer`) (`self.Damage`))
                (`KismetArrayLibrary.Array_AddUnique` (`self.HittedActors`) (`/Game/AI/SETUP/Blueprints/Utility/BFL_UtilitiesLibrary.GetPlayer`)))))))
      ;[1 1 1] Effect movement
      (`SceneComponent.K2_SetRelativeLocation` (`self.Niagara`) _returnvalue false false))
    (:`Finished`
      (`self.DestroySkill`))))

(fn `UserConstructionScript`
  (`parent.UserConstructionScript`))