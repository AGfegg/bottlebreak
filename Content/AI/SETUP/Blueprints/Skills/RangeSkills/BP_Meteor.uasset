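; Meteor range skill that drops from above the mouse cursor when used by the player, or above the player when used by an enemy.
; A cast of SkillOwner to BP_ParentAI selects the side, and gravity kicks in after a one-second delay.
; On impact, components overlapping the Cylinder are filtered to damage living enemies' HitBoxes or the player's HitBox.
; It then spawns two scaled explosions and destroys itself.
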(event `self.ReceiveBeginPlay`
  ;[1 1 1] Falling
  ;;[1 1 1] Who is skill owner?
  (cast `/Game/AI/SETUP/Blueprints/Character/BP_ParentAI` (`self.Skill_Owner`)
    (:`then`
      ;;[1 1 1] Calculate epicenter
      (`self.EpicenterIfUsedByPlayer`))
    (:`CastFailed`
      (`self.EpicenterIfUsedByEnemy`)))
  ;;[1 1 1] Fall after 1 second
  (`KismetSystemLibrary.Delay` 1.0)
  (set `ProjectileMovementComponent.ProjectileGravityScale` 5.0 (`self.ProjectileMovement`)))

(event `self.Box.OnComponentHit`
  (params (HitComponent :type "PrimitiveComponent Object Reference") (OtherActor :type "Actor Object Reference") (OtherComp :type "PrimitiveComponent Object Reference") (NormalImpulse :type "Vector Structure") (Hit :type "HitResult Structure (by ref)"))
  (bind _nextenemy (`self.NextEnemy`))
  (bind _returnvalue (`SceneComponent.K2_GetComponentLocation` (`self.Cylinder`)))
  ;[1 1 1] Get overlapping components after falling
  (for _array_element (`PrimitiveComponent.GetOverlappingComponents` (`self.Cylinder`))
    (set `self.NextComponent` _array_element)
    ;[1 1 1] Damage
    (cast `/Game/AI/SETUP/Blueprints/Character/BP_ParentAI` (`self.Skill_Owner`)
      (:`then`
        ;;[1 1 1] Used By Player
        ;;;[1 1 1] Ignore other actors
        (bind _asbp_enemy (cast `/Game/AI/SETUP/Blueprints/AI/BP_Enemy` (`ActorComponent.GetOwner` (`self.NextComponent`))))
        (set `self.NextEnemy` _asbp_enemy)
        ;;;[1 1 1] If meteor hit HitBox and enemy is not dead
        (if (and (== (`self.NextComponent`) (`/Game/AI/SETUP/Blueprints/AI/BP_Enemy.HitBox` _nextenemy)) (not (`/Game/AI/SETUP/Blueprints/AI/BP_Enemy.EnemyIsDead` _nextenemy)))
          ;;;[1 1 1] ...apply damage
          (`GameplayStatics.ApplyDamage` (`self.NextEnemy`) (`self.Damage`))))
      (:`CastFailed`
        ;;[1 1 1] Used By Enemy: if meteor hit player's HitBox - apply damage
        (if (== (`self.NextComponent`) (`/Game/AI/SETUP/Blueprints/Utility/BFL_UtilitiesLibrary.GetPlayersHitBox`))
          (`GameplayStatics.ApplyDamage` (`/Game/AI/SETUP/Blueprints/Utility/BFL_UtilitiesLibrary.GetPlayer`) (`self.Damage`))))))
  ;[1 1 1] Spawn effects
  (bind _returnvalue_2 (`NiagaraFunctionLibrary.SpawnSystemAtLocation` "/Game/AI/SETUP/Particles/P_Explosion.P_Explosion" _returnvalue))
  (`SceneComponent.SetRelativeScale3D` _returnvalue_2 (4.0 4.0 1.0))
  (bind _returnvalue_3 (`NiagaraFunctionLibrary.SpawnSystemAtLocation` "/Game/AI/SETUP/Particles/P_Explosion.P_Explosion" _returnvalue))
  (`SceneComponent.SetRelativeScale3D` _returnvalue_3 (3.0 3.0 3.0))
  ;[1 1 1] Destroy meteor
  (`self.DestroySkill`))

(fn `EpicenterIfUsedByEnemy`
  ;[1 1 1] Epicenter above player
  (`self.K2_SetActorLocation` (+ (`self.K2_GetActorLocation` (`GameplayStatics.GetPlayerCharacter` 0)) (0.0 0.0 500.0))))

(fn `EpicenterIfUsedByPlayer`
  ;[1 1 1] Epicenter above mouse cursor
  (`self.K2_SetActorLocation` (+ (`.Location` (`GameplayStatics.BreakHitResult` (`PlayerController.GetHitResultUnderCursorByChannel` (`GameplayStatics.GetPlayerController` 0) "TraceTypeQuery1" true))) (0.0 0.0 500.0))))

(fn `UserConstructionScript`
  (`parent.UserConstructionScript`))