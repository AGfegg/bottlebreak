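; Ranged light-shot skill projectile, usable by the player or enemies, that damages opposing hit boxes with an explosion effect.
; On spawn it aims at the player's target, or yaw-only toward the cursor; enemy shots aim at the player, then projectile movement is added.
; A SkillOwner cast to BP_ParentAI selects player behavior.
; It passes through victims, damaging each once via DamagedActors, and explodes when its Box hits or lifetime expires.
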(event `self.DamageSphere.OnComponentBeginOverlap`
  (params (OverlappedComponent :type "PrimitiveComponent Object Reference") (OtherActor :type "Actor Object Reference") (OtherComp :type "PrimitiveComponent Object Reference") (OtherBodyIndex :type Integer) (bFromSweep :type Boolean) (SweepResult :type "HitResult Structure (by ref)"))
  ;[1 1 1] Damage
  (set `self.NextActor` OtherActor)
  (set `self.NextComponent` OtherComp)
  ;;[1 1 1] Who is skill owner?
  (cast `/Game/AI/SETUP/Blueprints/Character/BP_ParentAI` (`self.Skill_Owner`)
    (:`then`
      ;;[1 1 1] Used by Player
      ;;;[1 1 1] Ignore other actors
      (bind _asbp_enemy (cast `/Game/AI/SETUP/Blueprints/AI/BP_Enemy` (`self.NextActor`)))
      ;;;[1 1 1] If DamageSphere hit enemy's HitBox and it's first hit
      (if (and (== (`/Game/AI/SETUP/Blueprints/AI/BP_Enemy.HitBox` _asbp_enemy) (`self.NextComponent`)) (not (`/Game/AI/SETUP/Blueprints/AI/BP_Enemy.EnemyIsDead` _asbp_enemy)))
        (if (== (`KismetArrayLibrary.Array_Find` (`self.DamagedActors`) (`self.NextActor`)) -1)
          ;;;[1 1 1] apply damage...
          (`GameplayStatics.ApplyDamage` (`self.NextActor`) (`self.Damage`))
          (`KismetArrayLibrary.Array_AddUnique` (`self.DamagedActors`) (`self.NextActor`))
          ;;;[1 1 1] and spawn effect.
          (bind _returnvalue (`NiagaraFunctionLibrary.SpawnSystemAtLocation` "/Game/AI/SETUP/Particles/P_Explosion.P_Explosion" (`self.K2_GetActorLocation` (`self.NextActor`))))
          (`SceneComponent.SetRelativeScale3D` _returnvalue (1.5 1.5 1.5)))))
    (:`CastFailed`
      ;;[1 1 1] Used by Enemy
      ;;;[1 1 1] If DamageSphere hit player's HitBox and it's first hit
      (if (== (`self.NextComponent`) (`/Game/AI/SETUP/Blueprints/Utility/BFL_UtilitiesLibrary.GetPlayersHitBox`))
        (if (== (`KismetArrayLibrary.Array_Find` (`self.DamagedActors`) (`self.NextActor`)) -1)
          ;;;[1 1 1] apply damage...
          (`GameplayStatics.ApplyDamage` (`self.NextActor`) (`self.Damage`))
          (`KismetArrayLibrary.Array_AddUnique` (`self.DamagedActors`) (`self.NextActor`))
          ;;;[1 1 1] and spawn effect.
          (bind _returnvalue_2 (`NiagaraFunctionLibrary.SpawnSystemAtLocation` "/Game/AI/SETUP/Particles/P_Explosion.P_Explosion" (`self.K2_GetActorLocation` (`self.NextActor`))))
          (`SceneComponent.SetRelativeScale3D` _returnvalue_2 (1.5 1.5 1.5)))))))

(event `self.ReceiveBeginPlay`
  (`|ExecutionSequence`
    (:`then_0`
      ;[1 1 1] Fireball Lifetime
      (`KismetSystemLibrary.Delay` (`self.FireballLifeTime`))
      (`NiagaraFunctionLibrary.SpawnSystemAtLocation` "/Game/AI/SETUP/Particles/P_Explosion.P_Explosion" (`self.K2_GetActorLocation`))
      (`self.DestroySkill`))
    (:`then_1`
      ;[1 1 1] Calculate direction for fireball
      (cast `/Game/AI/SETUP/Blueprints/Character/BP_ParentAI` (`self.Skill_Owner`)
        (:`then`
          (`self.LaunchByPlayer`) ; Fired by player
        )
        (:`CastFailed`
          (`self.LaunchByEnemy`) ; Fired by enemy
        )))))

(event `self.Box.OnComponentHit`
  (params (HitComponent :type "PrimitiveComponent Object Reference") (OtherActor :type "Actor Object Reference") (OtherComp :type "PrimitiveComponent Object Reference") (NormalImpulse :type "Vector Structure") (Hit :type "HitResult Structure (by ref)"))
  ;[1 1 1] Destroy on hit world static
  (bind _returnvalue (`NiagaraFunctionLibrary.SpawnSystemAtLocation` "/Game/AI/SETUP/Particles/P_Explosion.P_Explosion" (`self.K2_GetActorLocation`)))
  (`SceneComponent.SetRelativeScale3D` _returnvalue (1.5 1.5 1.5))
  (`self.DestroySkill`))

(fn `LaunchByEnemy`
  (bind _returnvalue (`self.K2_GetActorLocation` (`self.Skill_Owner`)))
  ;[1 1 1] Location and direction for enemy
  (`self.K2_AddActorLocalTransform` (`KismetMathLibrary.MakeTransform` (+ _returnvalue (0.0 0.0 30.0)) (`KismetMathLibrary.FindLookAtRotation` _returnvalue (+ (`self.K2_GetActorLocation` (`GameplayStatics.GetPlayerCharacter` 0)) (0.0 0.0 30.0)))))
  (`AddComponent|NODE_AddProjectileMovementComponent-2`))

(fn `LaunchByPlayer`
  (bind _returnvalue (`self.K2_GetActorLocation` (`GameplayStatics.GetPlayerCharacter` 0)))
  (bind _returnvalue_2 (`self.K2_GetActorLocation` (`GameplayStatics.GetPlayerCharacter` 0)))
  ;[1 1 1] Calculate direction if no enemy in target
  (if (!= (`/Game/AI/SETUP/Blueprints/Utility/BFL_UtilitiesLibrary.GetPlayersTarget`) null)
    ;[1 1 1] Calculate direction if enemy in target
    (`self.K2_AddActorLocalTransform` (`KismetMathLibrary.MakeTransform` (+ _returnvalue_2 (0.0 0.0 30.0)) (`KismetMathLibrary.FindLookAtRotation` _returnvalue_2 (+ (`self.K2_GetActorLocation` (`/Game/AI/SETUP/Blueprints/Utility/BFL_UtilitiesLibrary.GetPlayersTarget`)) (0.0 0.0 30.0)))))
    (`AddComponent|NODE_AddProjectileMovementComponent-1`)
    (else
      (`self.K2_AddActorLocalTransform` (`KismetMathLibrary.MakeTransform` (+ _returnvalue (0.0 0.0 30.0)) (`KismetMathLibrary.MakeRotator` 0.0 0.0 (.yaw (`KismetMathLibrary.FindLookAtRotation` _returnvalue (+ (`.Location` (`GameplayStatics.BreakHitResult` (`PlayerController.GetHitResultUnderCursorByChannel` (`GameplayStatics.GetPlayerController` 0) "TraceTypeQuery1" true))) (0.0 0.0 30.0)))))))
      (`AddComponent|NODE_AddProjectileMovementComponent-0`))))

(fn `UserConstructionScript`
  (`parent.UserConstructionScript`))