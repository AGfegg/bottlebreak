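; Static utility library for the AI and combat setup, giving shared access to player 0 (as BP_ParentAI) and BP_Enemy actors.
; Player helpers cover location, target, death and name-indexed stat arrays with clamped writes, printing errors on failure.
; CastSkill reads SkillsTable, deducts enemy mana or the player's cost stat, then spawns the skill actor at the origin for self-positioning.
; Enemy helpers toggle damage, rotation, task changes and custom-depth stencil outlines.
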(fn `allowDamage`
  (params (Enemy :type "Actor Object Reference") (Allow :type Boolean))
  (bind _asbp_enemy (cast `/Game/AI/SETUP/Blueprints/AI/BP_Enemy` Enemy)
    (:`then`
      (set `/Game/AI/SETUP/Blueprints/AI/BP_Enemy.DamageAvaliable` Allow _asbp_enemy))
    (:`CastFailed`
      (`KismetSystemLibrary.PrintString` null "AI is not inherited from BP_Enemy (Call from allowDamage)" true true (struct :`R` 1.0 :`A` 1.0)))))

(fn `allowRotation`
  (params (Enemy :type "Actor Object Reference") (Allow :type Boolean))
  (bind _asbp_enemy (cast `/Game/AI/SETUP/Blueprints/AI/BP_Enemy` Enemy)
    (:`then`
      (set `/Game/AI/SETUP/Blueprints/AI/BP_Enemy.RotationBlocked` (not Allow) _asbp_enemy))
    (:`CastFailed`
      (`KismetSystemLibrary.PrintString` null "AI is not inherited from BP_Enemy (Call from allowRotation)" true true (struct :`R` 1.0 :`A` 1.0)))))

(fn `allowTaskChange`
  (params (Enemy :type "Actor Object Reference") (Allow :type Boolean))
  (bind _asbp_enemy (cast `/Game/AI/SETUP/Blueprints/AI/BP_Enemy` Enemy)
    (:`then`
      (set `/Game/AI/SETUP/Blueprints/AI/BP_Enemy.RangeAttackInProgress` (not Allow) _asbp_enemy))
    (:`CastFailed`
      (`KismetSystemLibrary.PrintString` null "AI is not inherited from BP_Enemy (Call from allowTaskChange)" true true (struct :`R` 1.0 :`A` 1.0)))))

(fn `CastSkill`
  (params (SkillID :type Name) (Owner :type "Actor Object Reference"))
  (returns (Success :type Boolean) (Cooldown :type "Float (double-precision)"))
  (locals (SkillUsed :type Boolean :default true) (SkillCooldown :type "Float (double-precision)") (ID :type Name) (SkillOwner :type "Actor Object Reference") (SkillStats :type "/Game/AI/SETUP/Blueprints/Skills/Requirements Structure" :default (struct :`CostStat` "Mana")))
  (bind (_skillbp _name _description _coststat _cost) (break `/Game/AI/SETUP/Blueprints/Skills/Requirements` (`local.SkillStats`)))
  (bind (_skillbp_2 _name_2 _description_2 _coststat_2 _cost_2) (break `/Game/AI/SETUP/Blueprints/Skills/Requirements` (`local.SkillStats`)))
  (bind _value (`self.GetPlayersState` _coststat_2))
  ;[1 1 1] Initialize local variables
  (set `local.ID` SkillID)
  (set `local.SkillOwner` Owner)
  (bind _returnvalue (`|GetDataTableRow` "/Game/AI/SETUP/Blueprints/Skills/SkillsTable.SkillsTable" (`local.ID`))
    (:`then`
      (set `local.SkillStats` _returnvalue)
      ;[1 1 1] Who is caster?
      (bind _asbp_enemy (cast `/Game/AI/SETUP/Blueprints/AI/BP_Enemy` (`local.SkillOwner`))
        (:`then`
          (bind _statcurrent (`/Game/AI/SETUP/Blueprints/AI/BP_Enemy.StatCurrent` _asbp_enemy))
          (bind _output (`|GetArrayItem` _statcurrent 1))
          ;[1 1 1] Used by enemy
          (if (> _cost _output)
            ;[1 1 1] Failed
            (set `local.SkillUsed` false :!label _label)
            (else
              (`KismetArrayLibrary.Array_Set` _statcurrent 1 (- _output _cost))
              ;[1 1 1] Start mana regeration
              (`/Game/AI/SETUP/Blueprints/AI/BP_Enemy.ManaIsNotFull` _asbp_enemy)
              ;[1 1 1] Spawn skill-actor in 0.0.0 coordinate (should be moved to correct location in each skill blueprint)
              (bind _returnvalue_2 (`|SpawnActorFromClass` (`.SkillBP_10_EB7A910A42BD9CD4D3E38D90D57AFD9B` (break `/Game/AI/SETUP/Blueprints/Skills/Requirements` (`local.SkillStats`))) (`KismetMathLibrary.MakeTransform` (0.0 0.0 0.0)) "Undefined" "SelectDefaultAtRuntime" (`local.SkillOwner`) null :!label _label_2))
              (cast `/Game/AI/SETUP/Blueprints/Skills/BP_Skill` _returnvalue_2
                (:`then`
                  (set `local.SkillCooldown` (`.Cooldown_26_21EAC49F4FCFFD1923302D9146C48E27` (break `/Game/AI/SETUP/Blueprints/Skills/Requirements` (`local.SkillStats`)))))
                (:`CastFailed`
                  (goto _label))))))
        (:`CastFailed`
          ;[1 1 1] Used by player
          (if (> _cost_2 _value)
            (goto _label)
            (else
              (`self.SetPlayersState` (`.CostStat_17_EF0EA2DB40133811FAFDB28B4153E603` (break `/Game/AI/SETUP/Blueprints/Skills/Requirements` (`local.SkillStats`))) (- _value _cost_2))
              (goto _label_2))))))
    (:`RowNotFound`
      (goto _label)))
  (return (`local.SkillUsed`) (`local.SkillCooldown`)))

(fn `DistanceBetweenActorAndPlayer`
  (params (Actor :type "Actor Object Reference"))
  (returns (Distance :type "Float (double-precision)"))
  (return (`KismetMathLibrary.VSize` (- (`Actor.K2_GetActorLocation` Actor) (`Actor.K2_GetActorLocation` (`GameplayStatics.GetPlayerCharacter` null))))))

(fn `GetPlayer`
  (returns (playerRef :type "/Game/AI/SETUP/Blueprints/Character/BP_ParentAI Object Reference"))
  (bind _asbp_parent_ai (cast `/Game/AI/SETUP/Blueprints/Character/BP_ParentAI` (`GameplayStatics.GetPlayerCharacter` null))
    (:`then`
      (return _asbp_parent_ai))
    (:`CastFailed`
      (`KismetSystemLibrary.PrintString` null "Player is not inherited from CharacterBaseClass (Call from getPlayer)" true true (struct :`R` 1.0 :`A` 1.0))
      (return null))))

(fn `GetPlayersHitBox`
  (returns (HitBox :type "StaticMeshComponent Object Reference"))
  (bind _playerref (`self.GetPlayer` null))
  (`/Engine/EditorBlueprintResources/StandardMacros.IsValid` _playerref
    (:`Is Valid`
      (return (`/Game/AI/SETUP/Blueprints/Character/BP_ParentAI.HitSphere` _playerref)))
    (:`Is Not Valid`
      (`KismetSystemLibrary.PrintString` null "Invalid player reference (Call from getPlayersTarget)" true true (struct :`R` 1.0 :`A` 1.0))
      (return null))))

(fn `GetPlayersLocation`
  (returns (Location :type "Vector Structure"))
  (return (`Actor.K2_GetActorLocation` (`GameplayStatics.GetPlayerCharacter` null))))

(fn `GetPlayersState`
  (params (StatName :type Name))
  (returns (Value :type "Float (double-precision)"))
  (locals (StatValue :type "Float (double-precision)"))
  (bind _playerref (`self.GetPlayer` null))
  (bind _returnvalue (`KismetArrayLibrary.Array_Find` (`/Game/AI/SETUP/Blueprints/Character/BP_ParentAI.StatName` _playerref) StatName))
  (`/Engine/EditorBlueprintResources/StandardMacros.IsValid` _playerref
    (:`Is Valid`
      (if (== _returnvalue -1)
        (`KismetSystemLibrary.PrintString` null "Can't find stat" true true (struct :`R` 1.0 :`A` 1.0))
        (else
          ;[1 1 1] get value by index
          (set `local.StatValue` (`|GetArrayItem` (`/Game/AI/SETUP/Blueprints/Character/BP_ParentAI.StatCurrent` _playerref) _returnvalue))))
      (return (`local.StatValue`)))
    (:`Is Not Valid`
      (`KismetSystemLibrary.PrintString` null "Invalid player reference (Call from getPlayersStat)" true true (struct :`R` 1.0 :`A` 1.0))
      (return 0.0))))

(fn `GetPlayersStateMax`
  (params (StatName :type Name))
  (returns (Value :type "Float (double-precision)"))
  (locals (StatValue :type "Float (double-precision)"))
  (bind _playerref (`self.GetPlayer` null))
  (bind _returnvalue (`KismetArrayLibrary.Array_Find` (`/Game/AI/SETUP/Blueprints/Character/BP_ParentAI.StatName` _playerref) StatName))
  (`/Engine/EditorBlueprintResources/StandardMacros.IsValid` _playerref
    (:`Is Valid`
      (if (== _returnvalue -1)
        (`KismetSystemLibrary.PrintString` null "Can't find stat maximum" true true (struct :`R` 1.0 :`A` 1.0))
        (else
          ;[1 1 1] get value by index
          (set `local.StatValue` (`|GetArrayItem` (`/Game/AI/SETUP/Blueprints/Character/BP_ParentAI.StatMax` _playerref) _returnvalue))))
      (return (`local.StatValue`)))
    (:`Is Not Valid`
      (`KismetSystemLibrary.PrintString` null "Invalid player reference (Call from getPlayersStatMax)" true true (struct :`R` 1.0 :`A` 1.0))
      (return 0.0))))

(fn `GetPlayersStateMin`
  (params (StatName :type Name))
  (returns (Value :type "Float (double-precision)"))
  (locals (StatValue :type "Float (double-precision)"))
  (bind _playerref (`self.GetPlayer` null))
  (bind _returnvalue (`KismetArrayLibrary.Array_Find` (`/Game/AI/SETUP/Blueprints/Character/BP_ParentAI.StatName` _playerref) StatName))
  (`/Engine/EditorBlueprintResources/StandardMacros.IsValid` _playerref
    (:`Is Valid`
      (if (== _returnvalue -1)
        (`KismetSystemLibrary.PrintString` null "Can't find stat minimum" true true (struct :`R` 1.0 :`A` 1.0))
        (else
          ;[1 1 1] get value by index
          (set `local.StatValue` (`|GetArrayItem` (`/Game/AI/SETUP/Blueprints/Character/BP_ParentAI.StatMin` _playerref) _returnvalue))))
      (return (`local.StatValue`)))
    (:`Is Not Valid`
      (`KismetSystemLibrary.PrintString` null "Invalid player reference (Call from getPlayersStatMin)" true true (struct :`R` 1.0 :`A` 1.0))
      (return 0.0))))

(fn `GetPlayersTarget`
  (returns (TargetActor :type "Actor Object Reference"))
  (bind _playerref (`self.GetPlayer` null))
  (`/Engine/EditorBlueprintResources/StandardMacros.IsValid` _playerref
    (:`Is Valid`
      (return (`/Game/AI/SETUP/Blueprints/Character/BP_ParentAI.TargetActor` _playerref)))
    (:`Is Not Valid`
      (`KismetSystemLibrary.PrintString` null "Invalid player reference (Call from getPlayersTarget)" true true (struct :`R` 1.0 :`A` 1.0))
      (return null))))

(fn `GetPlayersTargetWidget`
  (returns (WidgetRef :type "/Game/AI/SETUP/UI/WB_TargetWidget Object Reference"))
  (bind _playerref (`self.GetPlayer` null))
  (`/Engine/EditorBlueprintResources/StandardMacros.IsValid` _playerref
    (:`Is Valid`
      (return (`/Game/AI/SETUP/Blueprints/Character/BP_ParentAI.TargetHUDWidget` _playerref)))
    (:`Is Not Valid`
      (`KismetSystemLibrary.PrintString` null "Invalid player reference (Call from getPlayersTargetWidget)" true true (struct :`R` 1.0 :`A` 1.0))
      (return null))))

(fn `GetRotationToPlayer`
  (params (Actor :type "Actor Object Reference"))
  (returns (Rot :type "Rotator Structure"))
  (return (`KismetMathLibrary.MakeRotator` 0.0 0.0 (.yaw (`KismetMathLibrary.FindLookAtRotation` (`Actor.K2_GetActorLocation` Actor) (`Actor.K2_GetActorLocation` (`GameplayStatics.GetPlayerCharacter` null)))))))

(fn `IsPlayerDead?`
  (returns (IsDead :type Boolean))
  (bind _playerref (`self.GetPlayer` null))
  (`/Engine/EditorBlueprintResources/StandardMacros.IsValid` _playerref
    (:`Is Valid`
      (return (`/Game/AI/SETUP/Blueprints/Character/BP_ParentAI.IsDead` _playerref)))
    (:`Is Not Valid`
      (`KismetSystemLibrary.PrintString` null "Invalid player reference (Call from isPlayerDead?)" true true (struct :`R` 1.0 :`A` 1.0))
      (return false))))

(fn `SetOutline`
  (params (ComponentForOutline :type "PrimitiveComponent Object Reference") (`On/Off` :type Boolean))
  (locals (Material :type "MaterialInstanceDynamic Object Reference") (Led :type Boolean) (Component :type "PrimitiveComponent Object Reference"))
  ;[1 1 1] Initialize local variables
  (set `local.Component` ComponentForOutline)
  (set `local.Led` `On/Off`)
  ;[1 1 1] Set outline if component is not equal to null
  (if (!= (`local.Component`) null)
    ;[1 1 1] You can add custom outline for each actor type here. Just connect logic to CastFailed
    (bind _asbp_enemy (cast `/Game/AI/SETUP/Blueprints/AI/BP_Enemy` (`ActorComponent.GetOwner` (`local.Component`))))
    ;[1 1 1] Works with Void Lantern Outliner. Disconnect StencilValue section, if your outline material is not working with stencils
    (`PrimitiveComponent.SetRenderCustomDepth` (`local.Component`) (`local.Led`))
    (`PrimitiveComponent.SetCustomDepthStencilValue` (`local.Component`) (`/Game/AI/SETUP/Blueprints/AI/BP_Enemy.OutlineColor` _asbp_enemy))))

(fn `SetPlayersState`
  (params (StatName :type Name) (Value :type "Float (double-precision)"))
  (bind _playerref (`self.GetPlayer` null))
  (bind _returnvalue (`KismetArrayLibrary.Array_Find` (`/Game/AI/SETUP/Blueprints/Character/BP_ParentAI.StatName` _playerref) StatName))
  (`/Engine/EditorBlueprintResources/StandardMacros.IsValid` _playerref
    (:`Is Valid`
      (if (== _returnvalue -1)
        (`KismetSystemLibrary.PrintString` null "Can't set stat - stat not found")
        (else
          (`KismetArrayLibrary.Array_Set` (`/Game/AI/SETUP/Blueprints/Character/BP_ParentAI.StatCurrent` _playerref) _returnvalue (`KismetMathLibrary.FClamp` Value (`|GetArrayItem` (`/Game/AI/SETUP/Blueprints/Character/BP_ParentAI.StatMin` _playerref) _returnvalue) (`|GetArrayItem` (`/Game/AI/SETUP/Blueprints/Character/BP_ParentAI.StatMax` _playerref) _returnvalue))))))
    (:`Is Not Valid`
      (`KismetSystemLibrary.PrintString` null "Invalid player reference (Call from setPlayersState)" true true (struct :`R` 1.0 :`A` 1.0)))))

(fn `SetPlayersTarget`
  (params (Actor :type "Actor Object Reference"))
  (bind _playerref (`self.GetPlayer` null))
  (`/Engine/EditorBlueprintResources/StandardMacros.IsValid` _playerref
    (:`Is Valid`
      (set `/Game/AI/SETUP/Blueprints/Character/BP_ParentAI.TargetActor` Actor _playerref))
    (:`Is Not Valid`
      (`KismetSystemLibrary.PrintString` null "Invalid player reference (Call from setPlayersTarget)" true true (struct :`R` 1.0 :`A` 1.0)))))