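; Enemy pack spawner that places a group of BP_Enemy AI at random navmesh points around itself on BeginPlay and manages them as a pack.
; Pack settings come from the SpawnersList DataTable by set or random ID, and enemies from NPCTable, either listed or randomly drawn.
; Each enemy keeps a spawner reference, while pack functions toggle shared chasing through Blackboards, restore health when chasing stops and destroy the spawner once the list empties.
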(event `self.ReceiveBeginPlay`
  (`self.Init`) ; Parameters initialization
  (`self.SpawnActors`) ; Spawn actors
)

(fn `Init`
  (bind _id (`self.ID`))
  (bind _possiblepackforrandomgen (`self.PossiblePackForRandomGen`))
  (`SceneComponent.SetVisibility` (`self.Cube`) false false)
  (if (`self.RandomPackFromSpawnersTable`)
    ;[1 1 1] Select random ID from PossiblePackForRandomGen-list and take parameters from row with selected ID
    (set `self.ID` (`|GetArrayItem` _possiblepackforrandomgen (`KismetMathLibrary.RandomIntegerInRange` 0 (- (`KismetArrayLibrary.Array_Length` _possiblepackforrandomgen) 1))))
    ;[1 1 1] Get parameters from row with certain ID
    (bind _returnvalue (`|GetDataTableRow` "/Game/AI/SETUP/Blueprints/AI/Datatable/SpawnersList.SpawnersList" (`self.ID`) :!label _label)
      (:`then`
        (set `self.Stats` _returnvalue))
      (:`RowNotFound`
        (`KismetSystemLibrary.PrintString` "Incorrect PackID in some spawner" true true (struct :`R` 0.62 :`G` 0.064334 :`A` 1.0))))
    (else
      ;[1 1 1] If ID = 0 ir None - spawn random enemies, set spawner parameters from 0 row of table
      (if (or (== _id "None") (== _id "0"))
        (bind _returnvalue_2 (`|GetDataTableRow` "/Game/AI/SETUP/Blueprints/AI/Datatable/SpawnersList.SpawnersList" "0")
          (:`then`
            (set `self.Stats` _returnvalue_2)))
        (else
          (goto _label))))))

(fn `IsPlayerInVisionOfAnyActor?`
  (returns (InVision :type Boolean))
  (locals (InVis :type Boolean))
  ;[1 1 1] Return true if any enemy in pack see player
  (for _array_element (`self.EnemyInPack`)
    (bind _asbp_enemy (cast `/Game/AI/SETUP/Blueprints/AI/BP_Enemy` _array_element)
      (:`then`
        (bind _distance (`/Game/AI/SETUP/Blueprints/Utility/BFL_UtilitiesLibrary.DistanceBetweenActorAndPlayer` _asbp_enemy))
        (if (<= _distance (`.EndChaseRange_45_3EA95C814C7DABE16D7312BD6290A72C` (break `/Game/AI/SETUP/Blueprints/AI/Datatable/NPCStats` (`/Game/AI/SETUP/Blueprints/AI/BP_Enemy.NPCStats` _asbp_enemy))))
          (return true)))
      (:`CastFailed`
        (`KismetSystemLibrary.PrintString` "One of the spawners has invalid Enemy class inside group" true true (struct :`R` 1.0 :`A` 1.0)))))
  (return false))

(fn `PlayerDetected`
  (locals (NextEnemy :type "/Game/AI/SETUP/Blueprints/AI/BP_Enemy Object Reference"))
  ;[1 1 1] Start chase for all enemies in pack if one see player
  (for _array_element (`self.EnemyInPack`)
    (bind _asbp_enemy (cast `/Game/AI/SETUP/Blueprints/AI/BP_Enemy` _array_element)
      (:`then`
        (bind _output_get (set `local.NextEnemy` _asbp_enemy))
        (bind _returnvalue (`AIBlueprintHelperLibrary.GetBlackboard` _output_get))
        (if (not (`BlackboardComponent.GetValueAsBool` _returnvalue "IsChasing"))
          (`BlackboardComponent.SetValueAsBool` _returnvalue "IsChasing" true)
          ;[1 1 1] Enable overlap events on Melee-Range for melee-enemies
          (if (`/Game/AI/SETUP/Blueprints/AI/BP_Enemy.IsMeleeEnemy` (`local.NextEnemy`))
            (set `PrimitiveComponent.bGenerateOverlapEvents` true (`/Game/AI/SETUP/Blueprints/AI/BP_Enemy.MeleeRange` (`local.NextEnemy`))))))
      (:`CastFailed`
        (`KismetSystemLibrary.PrintString` "One of the spawners has invalid Enemy class inside group" true true (struct :`R` 1.0 :`A` 1.0))))))

(fn `RemoveFromEnemyList`
  (params (Actor :type "Actor Object Reference"))
  (bind _enemyinpack (`self.EnemyInPack`))
  ;[1 1 1] Remove died enemy from enemy list and destroy spawner if list is empty
  (`KismetArrayLibrary.Array_RemoveItem` _enemyinpack Actor)
  (if (== (`KismetArrayLibrary.Array_LastIndex` _enemyinpack) -1)
    (`self.K2_DestroyActor`)))

(fn `SpawnActors`
  (bind _countofenemyforrandomgen (`self.CountOfEnemyForRandomGen`))
  (bind _possibleenemiesforrandomgen (`self.PossibleEnemiesForRandomGen`))
  (bind _id (`self.ID`))
  (bind (_monsteridlist _spawnrange) (break `/Game/AI/SETUP/Blueprints/AI/Datatable/Spawners` (`self.Stats`)))
  (if (or (== _id "None") (== _id "0"))
    (if (< _countofenemyforrandomgen 1)
      (`KismetSystemLibrary.PrintString` "Incorrect number of enemies for random generation" true true (struct :`R` 0.74 :`B` 0.027806 :`A` 1.0))
      (else
        (for _ (range 1 (+ _countofenemyforrandomgen 1))
          (bind _returnvalue (`|GetDataTableRow` "/Game/AI/SETUP/Blueprints/AI/Datatable/NPCTable.NPCTable" (`|GetArrayItem` _possibleenemiesforrandomgen (`KismetMathLibrary.RandomIntegerInRange` 0 (- (`KismetArrayLibrary.Array_Length` _possibleenemiesforrandomgen) 1))))
            (:`then`
              (bind (_enemyname _enemydescription _enemybp _behaviortree) (break `/Game/AI/SETUP/Blueprints/AI/Datatable/NPCStats` _returnvalue))
              (bind _returnvalue_2 (`AIBlueprintHelperLibrary.SpawnAIFromClass` _enemybp _behaviortree (`NavigationSystemV1.K2_GetRandomLocationInNavigableRadius` (`self.K2_GetActorLocation`) (`.SpawnRange_6_B3429D844FFC693DB97583B312DE5896` (break `/Game/AI/SETUP/Blueprints/AI/Datatable/Spawners` (`self.Stats`))) null null) (struct) true null))
              (bind _asbp_enemy (cast `/Game/AI/SETUP/Blueprints/AI/BP_Enemy` _returnvalue_2)
                (:`then`
                  (`self.K2_SetActorLocation` _asbp_enemy (+ (`self.K2_GetActorLocation` _asbp_enemy) (`KismetMathLibrary.MakeVector` 0.0 0.0 (`CapsuleComponent.GetScaledCapsuleHalfHeight` (`Character.CapsuleComponent` _asbp_enemy)))) false false)
                  (`KismetArrayLibrary.Array_AddUnique` (`self.EnemyInPack`) _asbp_enemy)
                  (set `/Game/AI/SETUP/Blueprints/AI/BP_Enemy.Spawner` self _asbp_enemy))
                (:`CastFailed`
                  (`KismetSystemLibrary.PrintString` "One of the row in NPCTable has invalid Enemy class" true true (struct :`R` 1.0 :`A` 1.0)))))
            (:`RowNotFound`
              (`KismetSystemLibrary.PrintString` "Incorrect EnemyID in some spawner" true true (struct :`R` 0.74 :`B` 0.027806 :`A` 1.0)))))))
    (else
      (for _array_element _monsteridlist
        (bind _returnvalue_3 (`|GetDataTableRow` "/Game/AI/SETUP/Blueprints/AI/Datatable/NPCTable.NPCTable" _array_element)
          (:`then`
            (bind (_enemyname_2 _enemydescription_2 _enemybp_2 _behaviortree_2) (break `/Game/AI/SETUP/Blueprints/AI/Datatable/NPCStats` _returnvalue_3))
            (bind _returnvalue_4 (`AIBlueprintHelperLibrary.SpawnAIFromClass` _enemybp_2 _behaviortree_2 (`NavigationSystemV1.K2_GetRandomLocationInNavigableRadius` (`self.K2_GetActorLocation`) _spawnrange null null) (struct) true null))
            (bind _asbp_enemy_2 (cast `/Game/AI/SETUP/Blueprints/AI/BP_Enemy` _returnvalue_4)
              (:`then`
                (`self.K2_SetActorLocation` _asbp_enemy_2 (+ (`self.K2_GetActorLocation` _asbp_enemy_2) (`KismetMathLibrary.MakeVector` 0.0 0.0 (`CapsuleComponent.GetScaledCapsuleHalfHeight` (`Character.CapsuleComponent` _asbp_enemy_2)))) false false)
                (`KismetArrayLibrary.Array_AddUnique` (`self.EnemyInPack`) _asbp_enemy_2)
                (set `/Game/AI/SETUP/Blueprints/AI/BP_Enemy.Spawner` self _asbp_enemy_2))
              (:`CastFailed`
                (`KismetSystemLibrary.PrintString` "One of the spawners has invalid Enemy class inside group" true true (struct :`R` 1.0 :`A` 1.0)))))
          (:`RowNotFound`
            (`KismetSystemLibrary.PrintString` "Incorrect enemy ID in some spawner" true true (struct :`R` 0.74 :`B` 0.027806 :`A` 1.0))))))))

(fn `StopChasingForAllActor`
  (locals (NextEnemy :type "/Game/AI/SETUP/Blueprints/AI/BP_Enemy Object Reference"))
  ;[1 1 1] Stop chase for all enemies in pack, restore health and disable overlap-event on melee range for melee-enemies
  (for _array_element (`self.EnemyInPack`)
    (bind _asbp_enemy (cast `/Game/AI/SETUP/Blueprints/AI/BP_Enemy` _array_element)
      (:`then`
        (bind _output_get (set `local.NextEnemy` _asbp_enemy))
        (`BlackboardComponent.SetValueAsBool` (`AIBlueprintHelperLibrary.GetBlackboard` _output_get) "IsChasing" false)
        (`MovementComponent.StopMovementImmediately` (`Character.CharacterMovement` (`local.NextEnemy`)))
        (`KismetArrayLibrary.Array_Set` (`/Game/AI/SETUP/Blueprints/AI/BP_Enemy.StatCurrent` (`local.NextEnemy`)) 0 (`.EnemyHealth_27_6CA6BFE444881DE6D5D02A88DEE50FB7` (break `/Game/AI/SETUP/Blueprints/AI/Datatable/NPCStats` (`/Game/AI/SETUP/Blueprints/AI/BP_Enemy.NPCStats` (`local.NextEnemy`)))))
        (if (`/Game/AI/SETUP/Blueprints/AI/BP_Enemy.IsMeleeEnemy` (`local.NextEnemy`))
          (set `PrimitiveComponent.bGenerateOverlapEvents` false (`/Game/AI/SETUP/Blueprints/AI/BP_Enemy.MeleeRange` (`local.NextEnemy`)))))
      (:`CastFailed`
        (`KismetSystemLibrary.PrintString` "One of the spawners has invalid Enemy class inside group" true true (struct :`R` 1.0 :`A` 1.0))))))

(fn `UserConstructionScript`)