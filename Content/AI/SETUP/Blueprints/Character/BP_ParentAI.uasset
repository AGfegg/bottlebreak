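; BP_ParentAI is a character Blueprint, named as an AI parent but built on player-style logic, with health, mana, energy and castable skills.
; BeginPlay maxes the stats, creates the player's bar and target widgets, and starts a looping mana regen timer.
; Damage reduces Health; at exactly zero, OnPlayerDied stops movement and disables player 0's input.
; Key 2 casts the second skill with a Delay-based cooldown; the other three skill chains are unwired.
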(event `self.ReceiveAnyDamage`
  (params (Damage :type "Float (single-precision)") (DamageType :type "DamageType Object Reference") (InstigatedBy :type "Controller Object Reference") (DamageCauser :type "Actor Object Reference"))
  ;[1 1 1] Taking damage from enemy
  (`/Game/AI/SETUP/Blueprints/Utility/BFL_UtilitiesLibrary.SetPlayersState` "Health" (- (`/Game/AI/SETUP/Blueprints/Utility/BFL_UtilitiesLibrary.GetPlayersState` "Health") Damage))
  (if (== (`/Game/AI/SETUP/Blueprints/Utility/BFL_UtilitiesLibrary.GetPlayersState` "Health") 0.0)
    ;[1 1 1] Player dead
    (`self.OnPlayerDied`)))

(event `self.ReceiveBeginPlay`
  (`|ExecutionSequence`
    (:`then_0`
      ;[1 1 1] Initialize variables
      (`self.Initialization`))
    (:`then_1`
      ;[1 1 1] Restore mana each second
      (`KismetSystemLibrary.K2_SetTimer` null "PassiveManaRegen" 1.0 true))))

(event `Key|One`
  (params (Key :type "Key Structure"))
  ;[1 1 1] Skill logic: use skill with ID from Skills array and set cooldown
)

(event `Key|Two`
  (params (Key :type "Key Structure"))
  ;[1 1 1] Skill logic: use skill with ID from Skills array and set cooldown
  (:`Pressed`
    ;;[1 1 1] If skill not in cooldown...
    (if (not (`self.Skill2Blocked`))
      ;;[1 1 1] ...cast skill...
      (bind (_success _cooldown) (`/Game/AI/SETUP/Blueprints/Utility/BFL_UtilitiesLibrary.CastSkill` (`|GetArrayItem` (`self.Skills`) 1) self))
      ;;[1 1 1] ...and set cooldown.
      (if _success
        (set `self.Skill2Blocked` true)
        (`KismetSystemLibrary.Delay` _cooldown)
        (set `self.Skill2Blocked` false)))))

(event `Key|RightMouseButton`
  (params (Key :type "Key Structure"))
  ;[1 1 1] Skill logic: use skill with ID from Skills array and set cooldown
)

(event `Key|Three`
  (params (Key :type "Key Structure"))
  ;[1 1 1] Skill logic: use skill with ID from Skills array and set cooldown
)

(fn `Initialization`
  (`|ExecutionSequence`
    (:`then_0`
      ;[1 1 1] Parameters initialization
      (`/Game/AI/SETUP/Blueprints/Utility/BFL_UtilitiesLibrary.SetPlayersState` "Health" (`/Game/AI/SETUP/Blueprints/Utility/BFL_UtilitiesLibrary.GetPlayersStateMax` "Health"))
      (`/Game/AI/SETUP/Blueprints/Utility/BFL_UtilitiesLibrary.SetPlayersState` "Mana" (`/Game/AI/SETUP/Blueprints/Utility/BFL_UtilitiesLibrary.GetPlayersStateMax` "Mana"))
      (`/Game/AI/SETUP/Blueprints/Utility/BFL_UtilitiesLibrary.SetPlayersState` "Energy" (`/Game/AI/SETUP/Blueprints/Utility/BFL_UtilitiesLibrary.GetPlayersStateMax` "Energy")))
    (:`then_1`
      ;[1 1 1] Creating TargetWidgen and PlayerBarWidget
      (bind _returnvalue (`|CreateWidget` "/Game/AI/SETUP/UI/WB_PlayerBarWidget.WB_PlayerBarWidget_C"))
      (bind _output_get (set `/Game/AI/SETUP/Blueprints/Character/BP_ParentAI.PlayerBarWidget` _returnvalue (`/Game/AI/SETUP/Blueprints/Utility/BFL_UtilitiesLibrary.GetPlayer`)))
      (`UserWidget.AddToViewport` _output_get 0))
    (:`then_2`
      (bind _returnvalue_2 (`|CreateWidget` "/Game/AI/SETUP/UI/WB_TargetWidget.WB_TargetWidget_C"))
      (bind _output_get_2 (set `/Game/AI/SETUP/Blueprints/Character/BP_ParentAI.TargetHUDWidget` _returnvalue_2 (`/Game/AI/SETUP/Blueprints/Utility/BFL_UtilitiesLibrary.GetPlayer`)))
      (`UserWidget.AddToViewport` _output_get_2 0))))

(fn `OnPlayerDied`
  (set `self.IsDead` true)
  (`self.DisableInput` (`GameplayStatics.GetPlayerCharacter` 0) (`GameplayStatics.GetPlayerController` 0))
  (`MovementComponent.StopMovementImmediately` (`self.CharacterMovement`)))

(fn `PassiveManaRegen`
  (bind _output (`|GetArrayItem` (`self.StatCurrent`) 1))
  ;[1 1 1] Restore 10 mana
  (if (< _output (`|GetArrayItem` (`self.StatMax`) 1))
    (`KismetArrayLibrary.Array_Set` (`self.StatCurrent`) 1 (`KismetMathLibrary.FClamp` (+ _output 10.0) (`|GetArrayItem` (`self.StatMin`) 1) (`|GetArrayItem` (`self.StatMax`) 1)))))

(fn `UserConstructionScript`)