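; Bottle spawner Blueprint that, on BeginPlay, spawns Bottle actors at the transforms of existing actors tagged "bottle".
; Each loop pass adds a tagged actor to MyBottleList, spawns at a random entry, then calls Remove and DestroyActor on random entries.
; Each Random lookup is separate, so those three steps can hit different actors.
; Bottle-count limit logic and random-point-in-box nodes are left disconnected.
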(event `self.ReceiveBeginPlay`
  (bind _outitem (`KismetArrayLibrary.Array_Random` (`self.MyBottleList`)))
  (bind _outactors (`GameplayStatics.GetAllActorsWithTag` "bottle"))
  (for _array_element _outactors
    (`KismetArrayLibrary.Array_Add` (`self.MyBottleList`) _array_element)
    (`|SpawnActorFromClass` "/Game/aliya/bottle.bottle_C" (`self.GetTransform` _outitem) "Undefined" "MultiplyWithRoot" null null)
    (`KismetArrayLibrary.Array_RemoveItem` (`self.MyBottleList`) _outitem)
    (`self.K2_DestroyActor` _outitem)))

(fn `UserConstructionScript`)